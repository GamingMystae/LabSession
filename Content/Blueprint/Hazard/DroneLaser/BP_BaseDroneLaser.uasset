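; BP_BaseDroneLaser is a drone laser projectile hazard that damages the player on impact.
; On BeginPlay it binds to the LaserMesh component's hit event, which spawns a Niagara burst at the impact point.
; If the hit actor casts to BP_ThirdPersonCharacter, it applies damage and destroys itself.
; Other hits only play the burst, because destruction sits behind the cast.
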(event Custom|OnComponentHit_Event
  (params (HitComponent :type Primitive%20Component%20Object%20Reference) (OtherActor :type Actor%20Object%20Reference) (OtherComp :type Primitive%20Component%20Object%20Reference) (NormalImpulse :type Vector) (Hit :type Hit%20Result%20Structure%20%28by%20ref%29))
  (bind (_bblockinghit _binitialoverlap _time _distance _location _impactpoint _normal _impactnormal _physmat _hitactor) (Collision|BreakHitResult Hit))
  ;[1 1 1] get the impact point, play vfx and destroy and apply damage to player
  (Niagara|SpawnSystematLocation "/Game/Assets/VFX/NS_LaserBigBurst.NS_LaserBigBurst" _impactpoint)
  (bind _asbp_third_person_character (Utilities|Casting|CastToBP_ThirdPersonCharacter _hitactor))
  (Default|ApplyDamage _asbp_third_person_character (Variables|Default|GetIn%20Damage%20Value))
  (Actor|DestroyActor))

(event EventBeginPlay
  ;[1 1 1] bind event on component hit
  (Collision|AssignOnComponentHit (Variables|Default|GetLaserMesh) (delegate Custom|OnComponentHit_Event)))

(event Collision|EventActorBeginOverlap
  (params (OtherActor :type Actor%20Object%20Reference))
  (|CallParentFunction OtherActor) ; This node is disabled and will not be called.\nDrag off pins to build functionality.
)

(event EventTick
  (params (DeltaSeconds :type Float%20%28single-precision%29))
  (|CallParentFunction DeltaSeconds) ; This node is disabled and will not be called.\nDrag off pins to build functionality.
)

(fn ConstructionScript
  (|CallParentFunction))