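; Spike-trap hazard that deals fixed damage through an inherited or shared OnDamage call to any actor overlapping its Box.
; BeginPlay caches the nail mesh's relative Z as the resting height.
; A SpikesAnimation timeline lerps the mesh Z from that height to a fixed target and plays the trap sound from an event track.
; Nothing in the graph starts the timeline, so it moves only if set to autoplay or triggered elsewhere.
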(event OnComponentBeginOverlap(Box)
  (params (OverlappedComponent :type Primitive%20Component%20Object%20Reference) (OtherActor :type Actor%20Object%20Reference) (OtherComp :type Primitive%20Component%20Object%20Reference) (OtherBodyIndex :type Integer) (bFromSweep :type Boolean) (SweepResult :type Hit%20Result%20Structure%20%28by%20ref%29))
  ;[1 1 1] Apply Damage
  (CallFunction|OnDamage OtherActor 15.0))

(event EventBeginPlay
  ;[1 1 1] On begin play set the Current Location with Z Value
  (|CallParentFunction)
  (Variables|Default|SetCurrentLocation (.z (Variables|/Script/Engine.SceneComponent|GetRelativeLocation (Variables|Default|GetNailsMesh)))))

(event Collision|EventActorBeginOverlap
  (params (OtherActor :type Actor%20Object%20Reference))
  (|CallParentFunction OtherActor) ; This node is disabled and will not be called.\nDrag off pins to build functionality.
)

(event EventTick
  (params (DeltaSeconds :type Float%20%28single-precision%29))
  (|CallParentFunction DeltaSeconds) ; This node is disabled and will not be called.\nDrag off pins to build functionality.
)

(fn ConstructionScript
  (|CallParentFunction))