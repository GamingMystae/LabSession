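; BP_Peaks is a hazard trap that fires a spike when the player enters its trigger area.
; The TriggerBox overlap calls ThrowSpike only when the overlapping actor is player character 0.
; ThrowSpike plays a sound at the trap and spawns a BP_PeakProjectile from the "Hole" socket on PeakBase, regardless of collision.
; No cooldown or one-shot guard exists, so each new overlap fires again.
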(event OnComponentBeginOverlap(TriggerBox)
  (params (OverlappedComponent :type Primitive%20Component%20Object%20Reference) (OtherActor :type Actor%20Object%20Reference) (OtherComp :type Primitive%20Component%20Object%20Reference) (OtherBodyIndex :type Integer) (bFromSweep :type Boolean) (SweepResult :type Hit%20Result%20Structure%20%28by%20ref%29))
  ;[1 1 1] Start the throw event
  (if (== OtherActor (Game|GetPlayerCharacter 0))
    (CallFunction|ThrowSpike)))

(event Custom|ThrowSpike
  ;[1 1 1] Event for fire the Spike
  (Audio|PlaySoundatLocation "/Engine/VREditor/Sounds/UI/Drop_Item_From_ContentBrowser.Drop_Item_From_ContentBrowser" (Transformation|GetActorLocation) "0, 0, 0" 1.0 1.0 0.0 0 0 0 0)
  (Game|SpawnActorfromClass "/Game/Blueprint/Hazard/Peak/BP_PeakProjectile.BP_PeakProjectile_C" (Transformation|GetSocketTransform (Variables|Default|GetPeakBase) "Hole" "RTS_World") "AlwaysSpawn" "MultiplyWithRoot" 0 0))

(event EventBeginPlay
  (|CallParentFunction) ; This node is disabled and will not be called.\nDrag off pins to build functionality.
)

(event Collision|EventActorBeginOverlap
  (params (OtherActor :type Actor%20Object%20Reference))
  (|CallParentFunction OtherActor) ; This node is disabled and will not be called.\nDrag off pins to build functionality.
)

(event EventTick
  (params (DeltaSeconds :type Float%20%28single-precision%29))
  (|CallParentFunction DeltaSeconds) ; This node is disabled and will not be called.\nDrag off pins to build functionality.
)

(fn ConstructionScript
  (|CallParentFunction))