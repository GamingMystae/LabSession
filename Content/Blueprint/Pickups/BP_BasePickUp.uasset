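; Base pickup actor that grants health, score and gold to the third-person player character on overlap.
; A timeline started on BeginPlay drives the root component's height and yaw for a floating, spinning animation.
; When BP_ThirdPersonCharacter enters the sphere, the pickup passes its three values to UpdatePickUpValues on the character, then destroys itself.
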(event OnComponentBeginOverlap(Sphere)
  (params (OverlappedComponent :type Primitive%20Component%20Object%20Reference) (OtherActor :type Actor%20Object%20Reference) (OtherComp :type Primitive%20Component%20Object%20Reference) (OtherBodyIndex :type Integer) (bFromSweep :type Boolean) (SweepResult :type Hit%20Result%20Structure%20%28by%20ref%29))
  ;[1 1 1] When the player overlaps call the update function
  (bind _asbp_third_person_character (Utilities|Casting|CastToBP_ThirdPersonCharacter OtherActor))
  (Default|UpdatePickUpValues _asbp_third_person_character (Variables|Default|GetIn%20Health) (Variables|Default|GetIn%20Score) (Variables|Default|GetIn%20Gold))
  (Actor|DestroyActor))

(event EventBeginPlay
  (bind _defaultsceneroot (Variables|Default|GetDefaultSceneRoot))
  (bind _relativelocation (Variables|/Script/Engine.SceneComponent|GetRelativeLocation _defaultsceneroot))
  ;[1 1 1] Spinning animation
  (bind (_direction _floating _rotation) (Timeline|Animation Play)
    (:Update
      (Transformation|SetRelativeLocationAndRotation _defaultsceneroot (Math|Vector|MakeVector (.x _relativelocation) (.y _relativelocation) _floating) (Math|Rotator|MakeRotator 0.0 0.0 _rotation) false false))))

(fn ConstructionScript)