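; Interactable door actor that swings open and closed, or reports that it is locked.
; OnInteract checks CanOpen, then plays a sound at the actor and uses a FlipFlop to alternate the RotateDoor timeline between play and reverse.
; The timeline's Angle track drives the relative yaw of the SMDoor component.
; When CanOpen is false, it only prints a locked-door message.
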(event EventBeginPlay
  (|CallParentFunction) ; This node is disabled and will not be called.\nDrag off pins to build functionality.
)

(event Collision|EventActorBeginOverlap
  (params (OtherActor :type Actor%20Object%20Reference))
  (|CallParentFunction OtherActor) ; This node is disabled and will not be called.\nDrag off pins to build functionality.
)

(event EventTick
  (params (DeltaSeconds :type Float%20%28single-precision%29))
  (|CallParentFunction DeltaSeconds) ; This node is disabled and will not be called.\nDrag off pins to build functionality.
)

(event EventOnInteract
  ;[1 1 1] Check if the player can open the door. if it true play sound and animation
  (if (Variables|Default|GetbCanOpen)
    (Audio|PlaySoundatLocation "/Engine/VREditor/Sounds/UI/Dockable_Window_Close.Dockable_Window_Close" (Transformation|GetActorLocation) "0, 0, 0" 1.0 1.0 0.0 0 0 0 0)
    (Utilities|FlowControl|FlipFlop
      (:A
        (bind _angle (Timeline|RotateDoor PlayFromStart)
          (:Update
            (Transformation|SetRelativeRotation (Variables|Default|GetSM_Door) (Math|Rotator|MakeRotator 0.0 0.0 _angle) false false))))
      (:B
        (Timeline|RotateDoor ReverseFromEnd)))
    (else
      (Development|PrintString "Locked Door"))))

(fn ConstructionScript
  (|CallParentFunction))