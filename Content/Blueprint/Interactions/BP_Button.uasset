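; BP_Button is a one-shot interactable button that opens a door when pressed.
; OnInteract sets IsPressed and plays a timeline that moves the SphereButton along Z, printing "Button Used" on any later interaction.
; When the animation finishes, it calls OpenDoor on the BP_BlockDoor2 found through GetActorOfClass, so the target door is looked up by class rather than by an assigned reference.
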(event EventBeginPlay
  (|CallParentFunction) ; This node is disabled and will not be called.\nDrag off pins to build functionality.
)

(event Collision|EventActorBeginOverlap
  (params (OtherActor :type Actor%20Object%20Reference))
  (|CallParentFunction OtherActor) ; This node is disabled and will not be called.\nDrag off pins to build functionality.
)

(event EventTick
  (params (DeltaSeconds :type Float%20%28single-precision%29))
  (|CallParentFunction DeltaSeconds) ; This node is disabled and will not be called.\nDrag off pins to build functionality.
)

(event EventOnInteract
  ;[1 1 1] Set the button to pressed, play animation
  (if (Variables|Default|GetbIsPressed)
    (Development|PrintString "Button Used")
    (else
      (Variables|Default|SetbIsPressed true)
      (bind _z_move (Timeline|PressAnimation Play)
        (:Update
          (Transformation|SetRelativeLocation (Variables|Default|GetSphereButton) (Math|Vector|MakeVector 0.0 0.0 _z_move) false false))
        (:Finished
          ;[1 1 1] Open the door
          (bind _returnvalue (Actor|GetActorOfClass "/Game/Blueprint/BlockDoor/BP_BlockDoor2.BP_BlockDoor2_C"))
          (Default|OpenDoor _returnvalue))))))

(fn ConstructionScript
  (|CallParentFunction))