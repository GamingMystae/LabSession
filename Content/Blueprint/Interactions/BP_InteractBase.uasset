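; BP_InteractBase is a base Blueprint for interactable objects that shows a widget when the player is near.
; The widget starts hidden on BeginPlay, and Sphere overlap events show or hide it, reacting only to player character 0.
; OnInteract is an empty event, so this file defines no interaction behavior of its own.
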(event OnComponentBeginOverlap(Sphere)
  (params (OverlappedComponent :type Primitive%20Component%20Object%20Reference) (OtherActor :type Actor%20Object%20Reference) (OtherComp :type Primitive%20Component%20Object%20Reference) (OtherBodyIndex :type Integer) (bFromSweep :type Boolean) (SweepResult :type Hit%20Result%20Structure%20%28by%20ref%29))
  ;[1 1 1] ON - OFF Widget
  ;;[1 1 1] Show widget on overlap
  (if (== OtherActor (Game|GetPlayerCharacter 0))
    (Development|SetHiddeninGame (Variables|Default|GetWidget) false false)))

(event OnComponentEndOverlap(Sphere)
  (params (OverlappedComponent :type Primitive%20Component%20Object%20Reference) (OtherActor :type Actor%20Object%20Reference) (OtherComp :type Primitive%20Component%20Object%20Reference) (OtherBodyIndex :type Integer))
  ;[1 1 1] ON - OFF Widget
  ;;[1 1 1] Hide widget on end overlap
  (if (== OtherActor (Game|GetPlayerCharacter 0))
    (Development|SetHiddeninGame (Variables|Default|GetWidget) true false)))

(event Custom|OnInteract)

(event EventBeginPlay
  ;[1 1 1] Inisialize widget hidden
  (Development|SetHiddeninGame (Variables|Default|GetWidget) true false))

(fn ConstructionScript)