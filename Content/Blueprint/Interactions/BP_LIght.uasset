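; BP_LIght is an interactable light that the player or another caller toggles on and off.
; It sets its PointLight to the LightOff intensity on BeginPlay.
; Each OnInteract call alternates through a FlipFlop between the LightOn and LightOff intensities, playing a button click sound at the actor's location.
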(event EventBeginPlay
  (|CallParentFunction)
  ;[1 1 1] initialize the intesity
  (Rendering|Components|Light|SetIntensity (Variables|Default|GetPointLight) (Variables|Default|GetLightOff)))

(event Collision|EventActorBeginOverlap
  (params (OtherActor :type Actor%20Object%20Reference))
  (|CallParentFunction OtherActor) ; This node is disabled and will not be called.\nDrag off pins to build functionality.
)

(event EventTick
  (params (DeltaSeconds :type Float%20%28single-precision%29))
  (|CallParentFunction DeltaSeconds) ; This node is disabled and will not be called.\nDrag off pins to build functionality.
)

(event EventOnInteract
  (bind _returnvalue (Transformation|GetActorLocation))
  ;[1 1 1] ON-OF Light
  (Utilities|FlowControl|FlipFlop
    (:A
      (Audio|PlaySoundatLocation "/Engine/VREditor/Sounds/UI/Click_on_Button.Click_on_Button" _returnvalue "0, 0, 0" 1.0 1.0 0.0 0 0 0 0)
      (Rendering|Components|Light|SetIntensity (Variables|Default|GetPointLight) (Variables|Default|GetLightOn)))
    (:B
      (Audio|PlaySoundatLocation "/Engine/VREditor/Sounds/UI/Click_on_Button.Click_on_Button" _returnvalue "0, 0, 0" 1.0 1.0 0.0 0 0 0 0)
      (Rendering|Components|Light|SetIntensity (Variables|Default|GetPointLight) (Variables|Default|GetLightOff)))))

(fn ConstructionScript
  (|CallParentFunction))