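; BP_DroneButton is a one-shot interactable button that destroys a referenced blue drone.
; On first interact it sets a pressed flag and plays a timeline that moves the button sphere along Z; later interactions only print a message.
; When the timeline finishes, it spawns an explosion effect and sound at the drone, destroys it, and notifies the room manager through DrownKilled.
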(event EventBeginPlay
  (|CallParentFunction) ; This node is disabled and will not be called.\nDrag off pins to build functionality.
)

(event Collision|EventActorBeginOverlap
  (params (OtherActor :type Actor%20Object%20Reference))
  (|CallParentFunction OtherActor) ; This node is disabled and will not be called.\nDrag off pins to build functionality.
)

(event EventTick
  (params (DeltaSeconds :type Float%20%28single-precision%29))
  (|CallParentFunction DeltaSeconds) ; This node is disabled and will not be called.\nDrag off pins to build functionality.
)

(event EventOnInteract
  (bind _bluedroneref (Variables|Default|GetBlueDroneRef))
  (bind _returnvalue (Transformation|GetActorTransform _bluedroneref))
  ;[1 1 1] when Interact set the IsPreesed to true . do the animation.
  (if (Variables|Default|GetbIsPressed)
    (Development|PrintString "Button Used")
    (else
      (Variables|Default|SetbIsPressed true)
      (bind _z_move (Timeline|Timeline Play)
        (:Update
          (Transformation|SetRelativeLocation (Variables|Default|GetSphereButton) (Math|Vector|MakeVector 0.0 0.0 _z_move) false false))
        (:Finished
          ;[1 1 1] when the animation finished Spawn emmiter and sound, destroy the drone and update the room manager
          (Niagara|SpawnSystematLocation "/Game/Assets/VFX/NS_BossExplosion.NS_BossExplosion" (.location _returnvalue) (.rotation _returnvalue) "7.000000,7.000000,7.000000")
          (Audio|PlaySoundatLocation "/Game/Assets/Sounds/Explosion_Cue.Explosion_Cue" (.location _returnvalue) "0, 0, 0" 4.0 1.0 0.0 0 0 0 0)
          (Actor|DestroyActor (Variables|Default|GetBlueDroneRef))
          (Default|DrownKilled (Variables|Default|GetManagerRef)))))))

(fn ConstructionScript
  (|CallParentFunction))