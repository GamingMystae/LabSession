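; Base drone actor that turns toward and flies at the player character, with support for firing big lasers from its rifle sockets.
; While StartBehavior is set, Tick smoothly interpolates look-at rotation and, if IsMoving, moves along the normalized direction to the player, scaled by delta time.
; SpawnLaserDown starts a looping timer that alternates left and right lower sockets, spawning a projectile, Niagara effect and sound.
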(event Custom|FireLaser
  ;[1 0.02604 0.02604] Spawn and fire laser
  ;;[1 1 1] Fire Left and right laser
  (Utilities|FlowControl|FlipFlop
    (:A
      (CallFunction|SpawnLaser (Variables|Default|GetSocketRifleLDown) (Variables|Default|GetBigLaserVfx) (Variables|Default|GetBP_LaserBig) (Variables|Default|GetSound)))
    (:B
      (CallFunction|SpawnLaser (Variables|Default|GetSocketRifleRDown) (Variables|Default|GetBigLaserVfx) (Variables|Default|GetBP_LaserBig) (Variables|Default|GetSound)))))

(event Custom|SpawnLaserDown
  ;[1 0.02604 0.02604] Spawn and fire laser
  ;;[1 1 1] Set the fire rate with timer
  (Utilities|Time|SetTimerbyEvent (delegate Custom|FireLaser) (Variables|Default|GetLaserFireTime) true))

(event Custom|SphereSocketDebug
  (bind _dronemesh (Variables|Default|GetDroneMesh))
  ;[0 0 0] Debug sphere for sockets visual
  (Utilities|FlowControl|Delay 2.0)
  (Rendering|Debug|DrawDebugSphere (Transformation|GetSocketLocation _dronemesh "RifleLup") 5.0 12 "(R=0.136347,G=0.076036,B=1.000000,A=1.000000)" 2.0)
  (Rendering|Debug|DrawDebugSphere (Transformation|GetSocketLocation _dronemesh "RifleLDown") 5.0 12 "(R=0.136347,G=0.076036,B=1.000000,A=1.000000)" 2.0)
  (Rendering|Debug|DrawDebugSphere (Transformation|GetSocketLocation _dronemesh "RifleLSmall") 5.0 12 "(R=0.136347,G=0.076036,B=1.000000,A=1.000000)" 2.0)
  (Rendering|Debug|DrawDebugSphere (Transformation|GetSocketLocation _dronemesh "RifleRup") 5.0 12 "(R=0.000000,G=1.000000,B=0.043550,A=1.000000)" 2.0)
  (Rendering|Debug|DrawDebugSphere (Transformation|GetSocketLocation _dronemesh "RifleRDown") 5.0 12 "(R=0.000000,G=1.000000,B=0.043550,A=1.000000)" 2.0)
  (Rendering|Debug|DrawDebugSphere (Transformation|GetSocketLocation _dronemesh "RifleRSmall") 5.0 12 "(R=0.000000,G=1.000000,B=0.043550,A=1.000000)" 2.0)
  (Rendering|Debug|DrawDebugSphere (Transformation|GetSocketLocation _dronemesh "BeamCenter") 1e+01 12 "(R=1.000000,G=0.000000,B=0.797707,A=1.000000)" 2.0))

(event EventBeginPlay
  (Variables|Default|SetPlayerRef (Game|GetPlayerCharacter 0))
  (Utilities|FlowControl|Delay 0.2))

(event EventTick
  (params (DeltaSeconds :type Float%20%28single-precision%29))
  ;[1 1 1] Check when to start the behavior
  (if (Variables|Default|GetStartBehavior)
    ;[1 1 1] interpolate location to target
    (CallFunction|InterpRotation DeltaSeconds (Variables|Default|GetInterp%20Speed))
    ;[1 1 1] check if the drone can move
    (if (and (Variables|Default|GetbIsMoving) (Variables|Default|GetStartBehavior))
      ;[1 1 1] Movement
      (CallFunction|MoveDronetoTarget (Variables|Default|GetSpeed)))))

(fn ConstructionScript)

(fn SpawnLaser
  (params (InSocketName :type Name) (SystemTemplate :type Niagara%20System%20Object%20Reference) (Class :type Actor%20Class%20Reference) (Sound :type Sound%20Base%20Object%20Reference))
  (bind _dronemesh (Variables|Default|GetDroneMesh))
  (bind _returnvalue (Transformation|GetSocketTransform _dronemesh InSocketName "RTS_World"))
  ;[1 1 1] Spawn the Laser class  from the socket
  (Game|SpawnActorfromClass Class (Transformation|GetSocketTransform (Variables|Default|GetDroneMesh) InSocketName "RTS_World") "AlwaysSpawn" "MultiplyWithRoot" 0 0)
  ;[1 1 1] Spawn the niagara system
  (Niagara|SpawnSystematLocation SystemTemplate (.location _returnvalue) (.rotation _returnvalue))
  (Audio|SpawnSoundatLocation Sound (Transformation|GetActorLocation) "0, 0, 0" 1.0 1.0 0.0 0 0))

(fn FindTargetRotation
  ;[1 1 1] Get Location
  (return (Math|Rotator|FindLookatRotation (Transformation|GetActorLocation) (Transformation|GetActorLocation (Variables|Default|GetPlayerRef)))))

(fn InterpRotation
  (params (InputPin :type Float%20%28single-precision%29) (InterpSpeed :type Float%20%28single-precision%29))
  ;[1 1 1] Take Charracter and drone location and use the look at rotation. So the drone always look at the character then set the rotation
  (Transformation|SetActorRotation (Math|Interpolation|RInterpTo (Transformation|GetActorRotation) (CallFunction|FindTargetRotation) InputPin InterpSpeed)))

(fn MoveDronetoTarget
  (params (MovementSpeed :type Integer))
  ;[1 1 1] Find the target location and start moving to it . Use delta seconds for independant frame rate
  (bind _output_get (Variables|Default|SetTargetLocation (CallFunction|FindtheTargetLocation)))
  (Transformation|AddActorWorldOffset (* (Utilities|Time|GetWorldDeltaSeconds) (* _output_get MovementSpeed))))

(fn FindtheTargetLocation
  ;[1 1 1] (Pure Function) subtract the vectors and the normilize it
  (return (Math|Vector|Normalize (- (Transformation|GetActorLocation (Variables|Default|GetPlayerRef)) (Transformation|GetActorLocation)))))