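; BP_BlockDoor2 is a door that opens by moving vertically when its OpenDoor event fires.
; BeginPlay caches the root component's starting relative Z.
; OpenDoor plays a rotate-loop sound at the actor's location and restarts the Movement timeline, which lerps the root's Z from the cached value to a fixed target height while keeping X and Y.
; The file contains no closing logic.
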(event Custom|OpenDoor
  (bind _defaultsceneroot (Variables|Default|GetDefaultSceneRoot))
  (bind _relativelocation (Variables|/Script/Engine.SceneComponent|GetRelativeLocation _defaultsceneroot))
  ;[1 1 1] Open the door
  (Audio|PlaySoundatLocation "/Engine/VREditor/Sounds/VR_objectRotateLoop_02_Cue.VR_objectRotateLoop_02_Cue" (Transformation|GetActorLocation) "0, 0, 0" 1.0 1.0 0.0 0 0 0 0)
  (bind _z_value (Timeline|Movement PlayFromStart)
    (:Update
      (Transformation|SetRelativeLocation (Variables|Default|GetDefaultSceneRoot) (Math|Vector|MakeVector (.x _relativelocation) (.y _relativelocation) (Math|Float|Lerp (Variables|Default|GetCurrentLocation) 5e+02 _z_value)) false false))))

(event EventBeginPlay
  ;[1 1 1] Inisialize value
  (Variables|Default|SetCurrentLocation (.z (Variables|/Script/Engine.SceneComponent|GetRelativeLocation (Variables|Default|GetDefaultSceneRoot)))))

(fn ConstructionScript)