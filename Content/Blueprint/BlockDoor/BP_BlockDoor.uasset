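; BP_BlockDoor is a trigger door that locks a room behind the player and activates the drones.
; When the player overlaps the Box, it disables the trigger's collision, plays a sound and runs a Timeline that lerps the door mesh's relative Z from its starting height to a fixed value.
; When the Timeline finishes, every BP_BaseDrone in the level gets StartBehavior set and SpawnLaserDown called.
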(event OnComponentBeginOverlap(Box)
  (params (OverlappedComponent :type Primitive%20Component%20Object%20Reference) (OtherActor :type Actor%20Object%20Reference) (OtherComp :type Primitive%20Component%20Object%20Reference) (OtherBodyIndex :type Integer) (bFromSweep :type Boolean) (SweepResult :type Hit%20Result%20Structure%20%28by%20ref%29))
  (bind _doormesh (Variables|Default|GetDoorMesh))
  (bind _relativelocation (Variables|/Script/Engine.SceneComponent|GetRelativeLocation _doormesh))
  ;[1 1 1] Lock the room
  ;;[1 1 1] Check if the actor is player
  (if (== OtherActor (Variables|Default|GetPlayerCharacter))
    ;;[1 1 1] Disable collision and play sound
    (Collision|SetCollisionEnabled (Variables|Default|GetBox) "NoCollision")
    (Audio|PlaySoundatLocation "/Game/Assets/Sounds/BlockDoor_Cue.BlockDoor_Cue" (Transformation|GetActorLocation) "0, 0, 0" 1.0 1.0 0.0 0 0 0 0)
    ;;[1 1 1] Play the animation
    (bind _z_value (Timeline|Timeline Play)
      (:Update
        (Transformation|SetRelativeLocation (Variables|Default|GetDoorMesh) (Math|Vector|MakeVector (.x _relativelocation) (.y _relativelocation) (Math|Float|Lerp (Variables|Default|GetCurrentLocation) 3.0 _z_value)) false false))
      (:Finished
        ;;[1 1 1] Get all the drones and start the behavior
        (bind _outactors (Actor|GetAllActorsOfClass "/Game/Blueprint/Drone/BP_BaseDrone.BP_BaseDrone_C"))
        (for _array_element _outactors
          (Variables|/Game/Blueprint/Drone/BP_BaseDrone.BP_BaseDrone_C|SetStartBehavior _array_element true)
          (Default|SpawnLaserDown _array_element))))))

(event EventBeginPlay
  ;[1 1 1] inisialize values
  (Variables|Default|SetPlayerCharacter (Game|GetPlayerCharacter 0))
  (Variables|Default|SetCurrentLocation (.z (Variables|/Script/Engine.SceneComponent|GetRelativeLocation (Variables|Default|GetDoorMesh)))))

(fn ConstructionScript)