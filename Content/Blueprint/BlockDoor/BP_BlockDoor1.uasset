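; BP_BlockDoor1 is a door actor that sinks out of the way when its UnlockDoor event is called.
; After a short delay it plays a sound at its location and runs a timeline that lowers DoorMesh on Z toward a fixed offset.
; Each update lerps from the mesh's current height rather than a stored start, so the motion compounds.
; The player character is cached at BeginPlay but not used here.
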(event Custom|UnlockDoor
  (bind _doormesh (Variables|Default|GetDoorMesh))
  (bind _relativelocation (Variables|/Script/Engine.SceneComponent|GetRelativeLocation _doormesh))
  ;[1 1 1] Event Unlock the door
  (Utilities|FlowControl|Delay 1.0)
  (Audio|PlaySoundatLocation "/Game/Assets/Sounds/BlockDoor_Cue.BlockDoor_Cue" (Transformation|GetActorLocation) "0, 0, 0" 1.0 1.0 0.0 0 0 0 0)
  (bind _z_value (Timeline|Timeline Play)
    (:Update
      (Transformation|SetRelativeLocation (Variables|Default|GetDoorMesh) (Math|Vector|MakeVector (.x _relativelocation) (.y _relativelocation) (Math|Float|Lerp (.z _relativelocation) -2e+02 _z_value)) false false))))

(event EventBeginPlay
  (Variables|Default|SetPlayerCharacter (Game|GetPlayerCharacter 0)))

(event Collision|EventActorBeginOverlap
  (params (OtherActor :type Actor%20Object%20Reference)))

(event EventTick
  (params (DeltaSeconds :type Float%20%28single-precision%29)))

(fn ConstructionScript)